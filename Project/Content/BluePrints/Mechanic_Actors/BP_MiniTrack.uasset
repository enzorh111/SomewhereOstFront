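; BP_MiniTrack is a track part that installs itself when its mesh overlaps a BP_AssemblyZone.
; The overlap sets the zone's Oruga flag, marking the track as present.
; The same actor then swaps its mesh to SM_Track, sets its relative transform, resets scale and stops simulating physics, with no attachment to the zone.
; A camera shutter sound plays at the zone's location as feedback.
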(event `self.StaticMesh.OnComponentBeginOverlap`
  (params (OverlappedComponent :type "PrimitiveComponent Object Reference") (OtherActor :type "Actor Object Reference") (OtherComp :type "PrimitiveComponent Object Reference") (OtherBodyIndex :type Integer) (bFromSweep :type Boolean) (SweepResult :type "HitResult Structure (by ref)"))
  (cast `/Game/BluePrints/Mechanic_Actors/BP_AssemblyZone` OtherActor)
  (bind _asbp_assembly_zone (cast `/Game/BluePrints/Mechanic_Actors/BP_AssemblyZone` OtherActor))
  (set `/Game/BluePrints/Mechanic_Actors/BP_AssemblyZone.Oruga` true _asbp_assembly_zone)
  (`StaticMeshComponent.SetStaticMesh` (`self.StaticMesh`) "/Game/Assets/CombinedStaticMesh/SM_Track.SM_Track")
  (`SceneComponent.K2_SetRelativeLocationAndRotation` :`self` (`self.StaticMesh`))
  (`PrimitiveComponent.SetSimulatePhysics` (`self.StaticMesh`) false)
  (`SceneComponent.SetRelativeScale3D` (`self.StaticMesh`) (1.0 1.0 1.0))
  (`GameplayStatics.PlaySoundAtLocation` "/Engine/VREditor/Sounds/UI/Camera_Shutter.Camera_Shutter" (`self.K2_GetActorLocation` _asbp_assembly_zone) (struct) 1.0 1.0 0.0 null null null null))

(fn `UserConstructionScript`)