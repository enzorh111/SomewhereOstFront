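; BP_AssemblyZone is an assembly zone actor that checks whether vehicle parts and ammunition are complete, then brings up the final interface.
; Each Tick it tests the Canon, Anillo, Rueda and Oruga flags and the BP_VRPawn's ammunition count.
; On success it spawns BI_Final_Interface at BI_Stats_Interface's transform and shrinks the latter at the origin, with no guard against repeating.
; Chassis checks and Spanish missing-part messages are unconnected.
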(event `self.ReceiveTick`
  (params (DeltaSeconds :type "Float (single-precision)"))
  (if (`self.Canon`)
    (if (`self.Anillo`)
      (if (`self.Rueda`)
        (if (`self.Oruga`)
          (bind _returnvalue (`GameplayStatics.GetActorOfClass` "/Game/BluePrints/VR/BP_VRPawn.BP_VRPawn_C"))
          (if (>= (`/Game/BluePrints/VR/BP_VRPawn.Ammunition` _returnvalue) 5)
            (bind _returnvalue_2 (`GameplayStatics.GetActorOfClass` "/Game/Interfaces/BI_Stats_Interface.BI_Stats_Interface_C"))
            (`|SpawnActorFromClass` "/Game/Interfaces/BI_Final_Interface.BI_Final_Interface_C" (`self.GetTransform` _returnvalue_2) "Undefined" "MultiplyWithRoot" null null)
            (`self.K2_SetActorTransform` _returnvalue_2 (`KismetMathLibrary.MakeTransform` (0.0 0.0 0.0) (struct) (0.001 0.001 0.001)) false false)))))))

(fn `UserConstructionScript`)